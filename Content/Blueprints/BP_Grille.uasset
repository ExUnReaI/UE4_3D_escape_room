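; BP_Grille is a grille actor that jumps to an open position once the player has opened a door.
; Every tick it casts the player to PLA_Character and, while DoorOpened is true, sets itself to a hardcoded location and rotation.
; After a one-second delay, a Bool flag lets a loud 2D iron hit sound play only once.
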(event EventTick
  (params (DeltaSeconds :type Float%20%28single-precision%29))
  (bind _aspla_character (Utilities|Casting|CastToPLA_Character (Game|GetPlayerCharacter 0)))
  (if (Variables|/Game/Blueprints/PLA_Character.PLA_Character_C|GetDoorOpened _aspla_character)
    (Transformation|SetActorLocation "1115.000000,136.000000,329.000000" false false)
    (Transformation|SetActorRotation "90.000000, 0, 0")
    (Utilities|FlowControl|Delay 1.0)
    (if (not (Variables|Default|Getbool))
      (Variables|Default|Setbool true)
      (Audio|PlaySound2D "/Game/Assets/SOUNDS/IronHit2.IronHit2" 4.0 1.0 0.0 0 0))))

(fn ConstructionScript)