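; BP_couvercle_coffre is a chest lid that rotates once when its Interact event fires.
; The construction script stores the lid's world roll as closed and adds 90 degrees for open.
; Interact sets two guard flags that are never reset, then plays a timeline in reverse from its end.
; The timeline lerps between both angles to set the lid's relative roll, zeroing pitch and yaw.
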(event EventInteract
  (if (not (Variables|Default|GetEnCours))
    (if (not (Variables|Default|GetChestOpened))
      (Variables|Default|SetChestOpened true)
      (Variables|Default|SetEnCours true)
      (bind _newtrack_0 (Timeline|Timeline_0 ReverseFromEnd)
        (:Update
          (Transformation|SetRelativeRotation (Variables|Default|Getcouvercle) (Math|Rotator|MakeRotator (Math|Float|Lerp (Variables|Default|GetRotaFerme) (Variables|Default|GetRotaOuvert) _newtrack_0) 0.0 0.0) false false))))))

(fn ConstructionScript
  (Variables|Default|SetRotaFerme (.roll (Transformation|GetWorldRotation (Variables|Default|Getcouvercle))))
  (Variables|Default|SetRotaOuvert (+ (Variables|Default|GetRotaFerme) 9e+01))
  (Variables|Default|SetEnCours false)
  (Variables|Default|SetChestOpened false))