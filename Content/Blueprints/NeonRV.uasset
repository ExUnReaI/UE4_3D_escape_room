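; NeonRV is an actor with a neon mesh that signals whether the player character is allowed to cross a red laser.
; On overlap it checks the PLA_Character's CanCrossRedLaser and CanCrossRedLaserEnd flags; either one switches the neon to ENeonV with a door lock sound.
; Otherwise it switches to ENeonR with an error sound.
; Any actor ending overlap restores the default ENeon material, as that event does no character check.
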(event Collision|EventActorBeginOverlap
  (params (OtherActor :type Actor%20Object%20Reference))
  (bind _neon (Variables|Default|Getneon))
  (bind _aspla_character (Utilities|Casting|CastToPLA_Character OtherActor))
  (if (Variables|/Game/Blueprints/PLA_Character.PLA_Character_C|GetCanCrossRedLaser _aspla_character)
    (Rendering|Material|SetMaterial _neon 0 "/Game/Assets/MATERIAUX/ENeonV.ENeonV" :!label _label)
    (Audio|PlaySound2D "/Game/Assets/SOUNDS/door_lock_turn_02.door_lock_turn_02" 1.0 1.0 0.0 0 0)
    (elif (Variables|/Game/Blueprints/PLA_Character.PLA_Character_C|GetCanCrossRedLaserEnd _aspla_character)
      (goto _label)
      (else
        (Rendering|Material|SetMaterial _neon 0 "/Game/Assets/MATERIAUX/ENeonR.ENeonR")
        (Audio|PlaySound2D "/Game/Assets/SOUNDS/Error.Error" 1.0 1.0 0.0 0 0)))))

(event Collision|EventActorEndOverlap
  (params (OtherActor :type Actor%20Object%20Reference))
  (Rendering|Material|SetMaterial (Variables|Default|Getneon) 0 "/Game/Assets/MATERIAUX/ENeon.ENeon"))

(fn ConstructionScript)