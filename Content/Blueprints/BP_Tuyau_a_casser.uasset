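; BP_Tuyau_a_casser is an interactable breakable pipe that only a player who owns the hammer can destroy.
; On Interact it casts the player to PLA_Character and checks HammerOwn, then plays a metal hit and destroys itself, or plays a negative grunt otherwise.
; An unconnected leftover branch would drop the cylinder with physics and play a one-time impact sound.
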(event EventInteract
  (bind _aspla_character (Utilities|Casting|CastToPLA_Character (Game|GetPlayerCharacter 0)))
  (if (Variables|/Game/Blueprints/PLA_Character.PLA_Character_C|GetHammerOwn _aspla_character)
    (Audio|PlaySound2D "/Game/Assets/SOUNDS/MetalHit.MetalHit" 1.0 1.0 0.0 0 0)
    (Actor|DestroyActor)
    (else
      (Audio|PlaySound2D "/Game/Assets/SOUNDS/Goblin_Negative_Grunt_2.Goblin_Negative_Grunt_2" 1.0 1.0 0.0 0 0))))

(fn ConstructionScript)