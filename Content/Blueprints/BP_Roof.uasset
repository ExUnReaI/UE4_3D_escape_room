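; BP_Roof is a roof actor that drops under physics once the player has opened a door.
; Each Tick it casts the player character to PLA_Character and polls its DoorOpened flag.
; The first time the flag is true, a Playedonce guard lets it play a 2D earthquake sound, enable physics simulation on the Roof component and greatly raise its mass scale.
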(event EventTick
  (params (DeltaSeconds :type Float%20%28single-precision%29))
  (bind _roof (Variables|Default|Getroof))
  (bind _aspla_character (Utilities|Casting|CastToPLA_Character (Game|GetPlayerCharacter 0)))
  (if (Variables|/Game/Blueprints/PLA_Character.PLA_Character_C|GetDoorOpened _aspla_character)
    (if (not (Variables|Default|Getplayedonce))
      (Variables|Default|Setplayedonce true)
      (Audio|PlaySound2D "/Game/Assets/SOUNDS/Earthquake.Earthquake" 0.7 0.8 2.0 0 0)
      (Physics|SetSimulatePhysics _roof true)
      (Class|PrimitiveComponent|SetMassScale _roof "None" 6e+02))))

(fn ConstructionScript)