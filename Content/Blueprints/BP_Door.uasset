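; BP_Door is a door actor that swings its Door component across a 90-degree yaw range when the player character's DoorActive flag is set.
; Tick polls that flag, and EnCours, never reset here, limits it to one trigger, which also sets DoorOpened on the character.
; A timeline played in reverse from its end lerps relative yaw between open and closed angles, which the construction script derives from world yaw.
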(event EventTick
  (params (DeltaSeconds :type Float%20%28single-precision%29))
  (bind _aspla_character (Utilities|Casting|CastToPLA_Character (Game|GetPlayerCharacter 0)))
  (if (Variables|/Game/Blueprints/PLA_Character.PLA_Character_C|GetDoorActive _aspla_character)
    (if (not (Variables|Default|GetEnCours))
      (Variables|/Game/Blueprints/PLA_Character.PLA_Character_C|SetDoorOpened _aspla_character true)
      (Variables|Default|SetEnCours true)
      (bind _newtrack_0 (Timeline|Timeline_0 ReverseFromEnd)
        (:Update
          (Transformation|SetRelativeRotation (Variables|Default|Getdoor) (Math|Rotator|MakeRotator 0.0 0.0 (Math|Float|Lerp (Variables|Default|GetRotaFerme) (Variables|Default|GetRotaOuvert) _newtrack_0)) false false))))))

(fn ConstructionScript
  (Variables|Default|SetRotaFerme (.yaw (Transformation|GetWorldRotation (Variables|Default|Getdoor))))
  (Variables|Default|SetRotaOuvert (- (Variables|Default|GetRotaFerme) 9e+01)))