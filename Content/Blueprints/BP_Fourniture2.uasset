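; BP_Fourniture2 is an interactable prop that the player can push once along the Y axis.
; Interact checks the player character's CanCrossRedLaser and CanPush flags, playing a negative grunt if either is false.
; A successful push sets IsMoving, which is never reset here, stores the starting Y and plays a metal creak.
; A timeline then lerps the actor's Y offset from zero to ValPousse.
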(event EventInteract
  (bind _returnvalue (Transformation|GetActorLocation))
  (bind _aspla_character (Utilities|Casting|CastToPLA_Character (Game|GetPlayerCharacter 0)))
  (if (Variables|/Game/Blueprints/PLA_Character.PLA_Character_C|GetCanCrossRedLaser _aspla_character)
    (if (Variables|/Game/Blueprints/PLA_Character.PLA_Character_C|GetCanPush _aspla_character)
      (if (not (Variables|Default|GetisMoving))
        (Variables|Default|SetisMoving true)
        (Variables|Default|SetValY (.y (Transformation|GetActorLocation)))
        (Audio|PlaySound2D "/Game/Assets/SOUNDS/metal_low_creaking_ship_structure_12.metal_low_creaking_ship_structure_12" 0.3 1.0 0.0 0 0)
        (bind _newtrack_0 (Timeline|Timeline_0 Play)
          (:Update
            (Transformation|SetActorRelativeLocation (Math|Vector|MakeVector (.x _returnvalue) (+ (Math|Float|Lerp 0.0 (Variables|Default|GetvalPousse) _newtrack_0) (Variables|Default|GetValY)) (.z _returnvalue))))))
      (else
        (Audio|PlaySound2D "/Game/Assets/SOUNDS/Goblin_Negative_Grunt_2.Goblin_Negative_Grunt_2" 0.4 1.0 0.0 0 0 :!label _label)))
    (else
      (goto _label))))

(fn ConstructionScript)