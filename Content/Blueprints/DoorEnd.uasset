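; DoorEnd is a neon-lit door, likely an end door, that opens only for a PLA_Character whose CanCrossRedLaserEnd flag is set.
; On overlap it swaps the neon material and plays a lock or error sound, then resets the neon when the overlap ends.
; A one-shot timeline lerps the door yaw 90 degrees from the closed rotation cached in the construction script, and the door never closes again.
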(event Collision|EventActorBeginOverlap
  (params (OtherActor :type Actor%20Object%20Reference))
  (bind _neon (Variables|Default|GetNeon))
  (bind _aspla_character (Utilities|Casting|CastToPLA_Character OtherActor))
  (if (Variables|/Game/Blueprints/PLA_Character.PLA_Character_C|GetCanCrossRedLaserEnd _aspla_character)
    (Rendering|Material|SetMaterial _neon 0 "/Game/Assets/MATERIAUX/ENeonV.ENeonV")
    (Audio|PlaySound2D "/Game/Assets/SOUNDS/door_lock_turn_02.door_lock_turn_02" 1.0 1.0 0.0 0 0)
    (if (not (Variables|Default|GetEnCours))
      (Variables|Default|SetEnCours true)
      (bind _newtrack_0 (Timeline|Timeline_0 Play)
        (:Update
          (Transformation|SetRelativeRotation (Variables|Default|Getdoor) (Math|Rotator|MakeRotator 0.0 0.0 (Math|Float|Lerp (Variables|Default|GetRotaFerme) (Variables|Default|GetRotaOuvert) _newtrack_0)) false false))))
    (else
      (Rendering|Material|SetMaterial _neon 0 "/Game/Assets/MATERIAUX/ENeonR.ENeonR")
      (Audio|PlaySound2D "/Game/Assets/SOUNDS/Error.Error" 1.0 1.0 0.0 0 0))))

(event Collision|EventActorEndOverlap
  (params (OtherActor :type Actor%20Object%20Reference))
  (Rendering|Material|SetMaterial (Variables|Default|GetNeon) 0 "/Game/Assets/MATERIAUX/ENeon.ENeon"))

(fn ConstructionScript
  (Variables|Default|SetRotaFerme (.yaw (Variables|/Script/Engine.SceneComponent|GetRelativeRotation (Variables|Default|GetDoor))))
  (Variables|Default|SetRotaOuvert (- (Variables|Default|GetRotaFerme) 9e+01)))