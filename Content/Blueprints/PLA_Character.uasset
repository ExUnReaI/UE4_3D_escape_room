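; First-person style player character with movement, look, mutually exclusive jump and crouch, and an M-key pause menu.
; Each tick, a short camera trace finds BPI_interact actors and sets InteractPossible, gating badge doors on badge ownership and furniture on push ability.
; E sends InteractMessage to the traced object when interaction is allowed.
; Tick also unlocks red laser crossings from collected part counts and plays a one-time camera shake when DoorOpened is set.
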(event Custom|Tick2
  ;[1 1 1] Interact
  (if (== (Variables|Default|GetPartLaser) 4.0)
    (Variables|Default|SetCanCrossRedLaser true))
  (if (== (Variables|Default|GetPartBadgeEnd) 8.0)
    (Variables|Default|SetCanCrossRedLaserEnd true))
  (if (Variables|Default|GetDoorOpened)
    (if (not (Variables|Default|GetdidOnce))
      (Variables|Default|SetdidOnce true)
      (Class|PlayerController|ClientPlayCameraShake (Game|GetPlayerController 0) "/Game/Blueprints/BP_CameraShake.BP_CameraShake_C" 2.5 "CameraLocal" "0, 0, 0"))))

(event EventTick
  (params (DeltaSeconds :type Float%20%28single-precision%29))
  (bind _camera (Variables|Default|GetCamera))
  (bind _returnvalue (Transformation|GetWorldLocation _camera))
  ;[1 1 1] Interact
  (CallFunction|Tick2)
  (bind _outhit (Collision|LineTraceByChannel _returnvalue (+ _returnvalue (* (Math|Vector|GetForwardVector _camera) 1.5e+02)) "TraceTypeQuery2" false 0 "None"))
  (Utilities|Casting|CastToBPI_interact (.HitActor (Collision|BreakHitResult _outhit))
    (:then
      (bind _output_get (Variables|Default|SetObject (.HitActor (Collision|BreakHitResult _outhit))))
      (if (== _output_get "/Game/Blueprints/BP_BadgeDoor.BP_BadgeDoor")
        (if (Variables|Default|GetBadgeOwn1)
          (Variables|Default|SetInteractPossible true)
          (else
            (Variables|Default|SetInteractPossible false)))
        (elif (== _output_get "/Game/Blueprints/BP_Fourniture.BP_Fourniture")
          (if (Variables|Default|GetCanPush)
            (Variables|Default|SetInteractPossible true)
            (else
              (Variables|Default|SetInteractPossible false)))
          (else
            (Variables|Default|SetInteractPossible true)))))
    (:CastFailed
      (Variables|Default|SetInteractPossible false))))

(event EventBeginPlay
  ;[1 1 1] Interact
  (bind _returnvalue (UserInterface|CreateWidget "/Game/HUD/InteractUI.InteractUI_C" (Game|GetPlayerController 0)))
  (UserInterface|Viewport|AddtoViewport _returnvalue 0))

(event Input|ActionEvents|InputActionCrouch
  (params (Key :type Key%20Structure))
  ;[1 1 1] Jump/crouch
  (:Pressed
    (if (Variables|Default|GetcanCrouch)
      (Character|Crouch)
      (Variables|Default|SetcanJump_1 false)))
  (:Released
    (Character|UnCrouch)
    (Variables|Default|SetcanJump_1 true)))

(event Input|ActionEvents|InputActionJump
  (params (Key :type Key%20Structure))
  ;[1 1 1] Jump/crouch
  (:Pressed
    (if (Variables|Default|GetcanJump_1)
      (Character|Jump)
      (Variables|Default|SetcanCrouch false)))
  (:Released
    (Variables|Default|SetcanCrouch true)))

(event Input|AxisEvents|InputAxisLook_left_right
  (params (AxisValue :type Float%20%28single-precision%29))
  ;[1 1 1] Camera
  (Pawn|Input|AddControllerYawInput AxisValue))

(event Input|AxisEvents|InputAxisLook_up_down
  (params (AxisValue :type Float%20%28single-precision%29))
  ;[1 1 1] Camera
  (Pawn|Input|AddControllerPitchInput AxisValue))

(event Input|AxisEvents|InputAxisMove_strafe
  (params (AxisValue :type Float%20%28single-precision%29))
  ;[1 1 1] Movement
  (if (== AxisValue 0.0)
    (Variables|Default|Setismoving false)
    (else
      (Variables|Default|Setismoving true)
      (Pawn|Input|AddMovementInput (Math|Vector|GetRightVector (Math|Rotator|MakeRotator 0.0 0.0 (.yaw (Pawn|GetControlRotation :!class /Script/Engine.Pawn)))) AxisValue false))))

(event Input|AxisEvents|InputAxisMove_forward
  (params (AxisValue :type Float%20%28single-precision%29))
  ;[1 1 1] Movement
  (if (== AxisValue 0.0)
    (Variables|Default|Setismoving false)
    (else
      (Variables|Default|Setismoving true)
      (Pawn|Input|AddMovementInput (Math|Vector|GetForwardVector (Math|Rotator|MakeRotator 0.0 0.0 (.yaw (Pawn|GetControlRotation :!class /Script/Engine.Pawn)))) AxisValue false))))

(event Input|KeyboardEvents|E
  (params (Key :type Key%20Structure))
  ;[1 1 1] Interact
  (:Pressed
    (if (Variables|Default|GetInteractPossible)
      (Class|BPIInteract|Interact(Message) (Variables|Default|GetObject)))))

(event Input|KeyboardEvents|M
  (params (Key :type Key%20Structure))
  ;[1 1 1] Menu Pause
  (:Pressed
    (Variables|/Script/Engine.PlayerController|SetbShowMouseCursor (Game|GetPlayerController 0) true)
    (Utilities|IsValid (Variables|Default|GetPause%20Menu%20Ref)
      (:Is%20Valid
        _)
      (:Is%20Not%20Valid
        (bind _returnvalue (UserInterface|CreateWidget "/Game/HUD/PauseMenu.PauseMenu_C"))
        (Variables|Default|SetPause%20Menu%20Ref _returnvalue)))
    (Input|SetInputModeUIOnly (Game|GetPlayerController 0) (Variables|Default|GetPause%20Menu%20Ref) "DoNotLock")
    (UserInterface|Viewport|AddtoViewport (Variables|Default|GetPause%20Menu%20Ref) 0)
    (Game|SetGamePaused true)))

(fn ConstructionScript
  (Variables|Default|SetBadgeOwn1 false)
  (Variables|Default|SetCanPush false)
  (Variables|Default|SetDoorActive false)
  (Variables|Default|SetInteractPossible false)
  (Variables|Default|SetBoostJump false)
  (Variables|Default|SetcanCrouch true)
  (Variables|Default|SetcanJump_1 true)
  (Variables|Default|SetPartLaser 0.0)
  (Variables|Default|SetPartBadgeEnd 0.0)
  (Variables|Default|SetCanCrossRedLaser false)
  (Variables|Default|SetCanCrossRedLaserEnd false))